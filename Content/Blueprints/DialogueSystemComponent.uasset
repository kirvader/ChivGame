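; Dialogue component that shows an NPC's conversations one line at a time in on-screen widgets.
; On BeginPlay it filters the NPCDIalogues data table by CurrentNPCID, starting a new conversation at each row numbered line 1.
; ShowNextLine replaces the current widget with a new DialogueWidget carrying the text from GetNextLine.
; GetNextLine advances conversation and line indices, returning empty text when a conversation ends, so no new widget appears.
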(event EventBeginPlay
  (CallFunction|GetAllConversations))

(event EventTick
  (params (DeltaSeconds :type Float%20%28single-precision%29)))

(fn ShowNextLine
  (Widget|RemovefromParent (Variables|Default|GetCurrentWidget))
  (bind _nextline (CallFunction|GetNextLine))
  (if (not (Utilities|Enum|Equal(Enum) _nextline (Utilities|Text|ToText(String) "")))
    (bind _returnvalue (UserInterface|CreateWidget (Variables|Default|GetDialogueWidget) (Game|GetPlayerController 0) _nextline))
    (bind _output_get (Variables|Default|SetCurrentWidget _returnvalue))
    (UserInterface|Viewport|AddtoViewport _output_get 0)))

(fn GetNextLine
  (if (== (Variables|Default|GetCurrentLineNumber) -1)
    (Math|Integer|IncrementInt (Variables|Default|GetCurrentConversationID)
      (:%20%20
        (Math|Integer|IncrementInt (Variables|Default|GetCurrentLineNumber)
          (:%20%20
            _))))
    (elif (== (Variables|Default|GetCurrentLineNumber) (Utilities|Array|LastIndex (Utilities|Struct|BreakStructure_Conversation (Utilities|Array|Get(acopy) (Variables|Default|GetConversations) (Variables|Default|GetCurrentConversationID)))))
      (Variables|Default|SetCurrentLineNumber -1)
      (if (== (Variables|Default|GetCurrentConversationID) (Utilities|Array|LastIndex (Variables|Default|GetConversations)))
        _
        (else
          (Math|Integer|IncrementInt (Variables|Default|GetCurrentConversationID)
            (:%20%20
              _))))
      (else
        (Math|Integer|IncrementInt (Variables|Default|GetCurrentLineNumber)
          (:%20%20
            _)))))
  (if (== (Variables|Default|GetCurrentLineNumber) -1)
    (return "")
    (else
      (return (Utilities|Array|Get(acopy) (Utilities|Struct|BreakStructure_Conversation (Utilities|Array|Get(acopy) (Variables|Default|GetConversations) (Variables|Default|GetCurrentConversationID))) (Variables|Default|GetCurrentLineNumber))))))

(fn GetAllConversations
  (bind _conversations (Variables|Default|GetConversations))
  (bind _outrownames (DataTable|GetDataTableRowNames "/Game/GameInstances/DataTables/NPCDIalogues.NPCDIalogues"))
  (for _array_element _outrownames
    (bind _returnvalue (Utilities|GetDataTableRow "/Game/GameInstances/DataTables/NPCDIalogues.NPCDIalogues" _array_element)
      (:then
        (if (== (.NPC_ID (Utilities|Struct|BreakStructure_Dialogue _returnvalue)) (Variables|Default|GetCurrentNPCID))
          (if (== (.LineNumber (Utilities|Struct|BreakStructure_Dialogue _returnvalue)) 1)
            (Utilities|Array|Add (Variables|Default|GetConversations) (Utilities|Struct|MakeStructure_Conversation)))
          (Utilities|Array|Add (Utilities|Struct|BreakStructure_Conversation (Utilities|Array|Get(acopy) _conversations (Utilities|Array|LastIndex _conversations))) (.LineText (Utilities|Struct|BreakStructure_Dialogue _returnvalue))))))))